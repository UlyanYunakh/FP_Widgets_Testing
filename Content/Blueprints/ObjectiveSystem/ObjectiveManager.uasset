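; ObjectiveManager spawns gameplay objectives at locations read from the level's ObjectiveList actor, offset by that actor's world position.
; The first four TestObjective actors appear sequentially, each bound completion removing the current objective and advancing the index.
; After those, all remaining objectives spawn at once without a completion binding.
; OnObjectiveAdd and OnObjectiveRemove dispatchers broadcast the changes to listeners.
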(event Custom|NewObjective
  (params (Index :type Integer))
  (if (< Index 4)
    (bind _output_get (Variables|Default|SetCurrentObjective Index))
    (bind _returnvalue (Game|SpawnActorfromClass "/Game/Blueprints/Levels/MarkerWidgetShowcase/TestObjective.TestObjective_C" (Math|Transform|MakeTransform (Utilities|Array|Get(acopy) (Variables|Default|GetLocations) _output_get) "0, 0, 0" "1,1,1") "Undefined" 0 0))
    (Default|CallOnObjectiveAdd _returnvalue (Variables|Default|GetCurrentObjective))
    (EventDispatchers|AssignObjectiveComplite _returnvalue (delegate Custom|OnComplite))
    (else
      (for (_array_element _array_index) (Variables|Default|GetLocations)
        (if (>= _array_index 4)
          (bind _returnvalue_2 (Game|SpawnActorfromClass "/Game/Blueprints/Levels/MarkerWidgetShowcase/TestObjective.TestObjective_C" (Math|Transform|MakeTransform _array_element "0, 0, 0" "1,1,1") "Undefined" 0 0))
          (Default|CallOnObjectiveAdd _returnvalue_2 _array_index))))))

(event Custom|OnComplite
  (Default|CallOnObjectiveRemove (Variables|Default|GetCurrentObjective))
  (bind _output_get (Variables|Default|SetCurrentObjective (+ (Variables|Default|GetCurrentObjective) 1)))
  (CallFunction|NewObjective _output_get))

(event EventBeginPlay
  (Utilities|FlowControl|Delay 0.2)
  (bind _returnvalue (Actor|GetActorOfClass "/Game/Blueprints/Levels/MarkerWidgetShowcase/ObjectiveList.ObjectiveList_C"))
  (for _array_element (Variables|/Game/Blueprints/Levels/MarkerWidgetShowcase/ObjectiveList.ObjectiveList_C|GetLocations _returnvalue)
    (Utilities|Array|Add (Variables|Default|GetLocations) (+ _array_element (Transformation|GetWorldLocation (Variables|/Game/Blueprints/Levels/MarkerWidgetShowcase/ObjectiveList.ObjectiveList_C|GetDefaultSceneRoot _returnvalue)))))
  (CallFunction|NewObjective))

(fn ConstructionScript)