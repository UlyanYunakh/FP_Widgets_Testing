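; Pawn component that shows interaction widgets on nearby FP_Toggle_Actors the owner can see.
; On BeginPlay it adds a collision volume sized by the visibility range; overlaps activate actors and track them in an array, and exits deactivate and hide them.
; Each Tick, tracked actors within screen bounds get a visibility line trace from the owner's eyes, showing the widget only if that actor is hit first.
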(event EventBeginPlay
  (CallFunction|FPCreateCollisionComponent))

(event EventTick
  (params (DeltaSeconds :type Float%20%28single-precision%29))
  (CallFunction|FPCheckVisibilityOfIteractables))

(fn FPCheckVisibilityOfIteractables
  (bind _isempty (CallFunction|FPIsArrayEmpty (Variables|Default|GetFP_InteractActorsNearBy)))
  (if (not _isempty)
    (for _array_element (Variables|Default|GetFP_InteractActorsNearBy)
      (if (Variables|/Game/Blueprints/FP_Toggle_ActorComponent.FP_Toggle_ActorComponent_C|GetFP_IsInScreenBounds (Variables|/Game/Blueprints/FP_Toggle_Actor.FP_Toggle_Actor_C|GetFP_Interact_Actor_Component _array_element))
        (LocalVariables|SetFP_CurrentIteractable _array_element)
        (bind _outhit (Collision|LineTraceByChannel (.OutLocation (Actor|GetActorEyesViewPoint (Components|GetOwner))) (Transformation|GetActorLocation (LocalVariables|GetFP_CurrentIteractable)) "TraceTypeQuery1" false 0 "None"))
        (bind _asfp_interact_actor (Utilities|Casting|CastToFP_Toggle_Actor (.hitactor _outhit))
          (:then
            (Default|FPToggleWidgetVisibility (Variables|/Game/Blueprints/FP_Toggle_Actor.FP_Toggle_Actor_C|GetFP_Interact_Actor_Component (LocalVariables|GetFP_CurrentIteractable)) (== _asfp_interact_actor (LocalVariables|GetFP_CurrentIteractable))))
          (:CastFailed
            (Default|FPToggleWidgetVisibility (Variables|/Game/Blueprints/FP_Toggle_Actor.FP_Toggle_Actor_C|GetFP_Interact_Actor_Component (LocalVariables|GetFP_CurrentIteractable)) false)))))
    (return)))

(fn FPonCollisionBeginOverlap
  (params (OverlappedComponent :type Primitive%20Component%20Object%20Reference) (OtherActor :type Actor%20Object%20Reference) (OtherComp :type Primitive%20Component%20Object%20Reference) (OtherBodyIndex :type Integer) (bFromSweep :type Boolean) (SweepResult :type Hit%20Result%20Structure%20%28by%20ref%29))
  (bind _asfp_interact_actor (Utilities|Casting|CastToFP_Toggle_Actor OtherActor))
  (Variables|/Game/Blueprints/FP_Toggle_ActorComponent.FP_Toggle_ActorComponent_C|SetFP_IsActivated (Variables|/Game/Blueprints/FP_Toggle_Actor.FP_Toggle_Actor_C|GetFP_Interact_Actor_Component _asfp_interact_actor) true)
  (Utilities|Array|Add (Variables|Default|GetFP_InteractActorsNearBy) _asfp_interact_actor)
  (return))

(fn FPCreateCollisionComponent
  (bind _fp_collision (CallFunction|FPAddCollisiontoActor (Components|GetOwner) (Variables|Default|GetFP_VisibilityRange)))
  (bind _output_get (Variables|Default|SetFP_VisibilityCollision _fp_collision))
  (Collision|BindEventtoOnComponentBeginOverlap _output_get (EventDispatchers|CreateEvent :!event FPonCollisionBeginOverlap))
  (Collision|BindEventtoOnComponentEndOverlap _output_get (EventDispatchers|CreateEvent :!event FPonCollisionEndOverlap))
  (return))

(fn FPonCollisionEndOverlap
  (params (OverlappedComponent :type Primitive%20Component%20Object%20Reference) (OtherActor :type Actor%20Object%20Reference) (OtherComp :type Primitive%20Component%20Object%20Reference) (OtherBodyIndex :type Integer))
  (bind _asfp_interact_actor (Utilities|Casting|CastToFP_Toggle_Actor OtherActor))
  (Variables|/Game/Blueprints/FP_Toggle_ActorComponent.FP_Toggle_ActorComponent_C|SetFP_IsActivated (Variables|/Game/Blueprints/FP_Toggle_Actor.FP_Toggle_Actor_C|GetFP_Interact_Actor_Component _asfp_interact_actor) false)
  (Default|FPToggleWidgetVisibility (Variables|/Game/Blueprints/FP_Toggle_Actor.FP_Toggle_Actor_C|GetFP_Interact_Actor_Component _asfp_interact_actor) false)
  (Utilities|Array|RemoveItem (Variables|Default|GetFP_InteractActorsNearBy) _asfp_interact_actor)
  (return))