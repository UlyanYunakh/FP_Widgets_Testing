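; FP_Toggle_FuncHelper is a set of helper functions, apparently supporting an FP toggle system.
; It derives box points by reflecting the extent across a set of normals and offsetting by the origin.
; Other helpers add a sphere component of given radius to an actor, test whether an array is empty, and return viewport bounds inset by a padding value.
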(fn FPGetBoxTops
  (params (BoxOrigin :type Vector) (BoxExtent :type Vector))
  (for _array_element (LocalVariables|GetnormalsArray)
    (Utilities|Array|Add (LocalVariables|GettopsArray) (+ (Math|Vector|GetReflectionVector BoxExtent _array_element) BoxOrigin)))
  (return (LocalVariables|GettopsArray)))

(fn FPAddCollisiontoActor
  (params (FP_Actor :type Actor%20Object%20Reference) (FP_Radius :type Float%20%28single-precision%29))
  (bind _returnvalue (Game|AddComponentbyClass FP_Actor "/Script/Engine.SphereComponent" false))
  (Components|Sphere|SetSphereRadius _returnvalue FP_Radius true)
  (return _returnvalue))

(fn FPIsArrayEmpty
  (params (FP_Array :type Array%20of%20Object%20Object%20References))
  (return (< (Utilities|Array|Length FP_Array) 1)))

(fn FPGetAvailableScreenSpace
  (bind ___worldcontext (LocalVariables|Get__WorldContext))
  (bind _fp_padding (LocalVariables|GetFP_Padding))
  (bind _returnvalue (Viewport|GetViewportSize ___worldcontext))
  (return _fp_padding (- (.x _returnvalue) _fp_padding) _fp_padding (- (.y _returnvalue) _fp_padding)))