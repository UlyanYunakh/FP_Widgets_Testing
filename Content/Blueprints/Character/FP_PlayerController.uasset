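; First-person player controller that caches the possessed FP_Character and passes it movement and camera input.
; Movement axes become yaw-only forward and right vectors from control rotation before reaching the character's OnMovement, while pitch and yaw go to OnCameraMovement.
; Tick runs a profile line trace whose result is unused.
; An uncalled debug function projects nearby interactables to screen space and prints whether each lies within the viewport.
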(event EventTick
  (params (DeltaSeconds :type Float%20%28single-precision%29))
  (Class|KismetSystemLibrary|LineTraceSinglebyProfile "0, 0, 0" "0, 0, 0" "None" false 0 "None" true))

(event EventPossess
  (params (PossessedPawn :type Pawn%20Object%20Reference))
  ;[1 1 1] Save possessed pawn as variable
  (bind _asfp_character (Utilities|Casting|CastToFP_Character PossessedPawn))
  (Variables|Default|SetPossessedPawn _asfp_character))

(event Input|AxisEvents|InputAxisMoveForward
  (params (AxisValue :type Float%20%28single-precision%29))
  ;[1 1 1] Movement input event listeners
  (CallFunction|HandleCharecterMovement AxisValue "NewEnumerator0"))

(event Input|AxisEvents|InputAxisMoveRight
  (params (AxisValue :type Float%20%28single-precision%29))
  ;[1 1 1] Movement input event listeners
  (CallFunction|HandleCharecterMovement AxisValue "NewEnumerator1"))

(event Input|AxisEvents|InputAxisCameraPitch
  (params (AxisValue :type Float%20%28single-precision%29))
  ;[1 1 1] Camera movement event listener
  (CallFunction|HandleCameraMovement "NewEnumerator0" AxisValue))

(event Input|AxisEvents|InputAxisCameraYaw
  (params (AxisValue :type Float%20%28single-precision%29))
  ;[1 1 1] Camera movement event listener
  (CallFunction|HandleCameraMovement "NewEnumerator1" AxisValue))

(fn ConstructionScript)

(fn HandleCharecterMovement
  (params (Scale :type Float%20%28single-precision%29) (Direction :type FP_MovementDirection%20Enum :default "NewEnumerator0"))
  (bind _returnvalue (Pawn|GetControlRotation :!class /Script/Engine.Controller))
  (bind _yaw (Math|Rotator|BreakRotator _returnvalue))
  (bind _returnvalue_2 (Math|Rotator|MakeRotator 0.0 0.0 _yaw))
  (switch Utilities|FlowControl|Switch|SwitchonFP_MovementDirection Direction
    (:NewEnumerator0
      (LocalVariables|SetDirectionVector (Math|Vector|GetForwardVector _returnvalue_2)))
    (:NewEnumerator1
      (LocalVariables|SetDirectionVector (Math|Vector|GetRightVector _returnvalue_2))))
  (Default|OnMovement (Variables|Default|GetPossessedPawn) (LocalVariables|GetDirectionVector) Scale)
  (return))

(fn HandleCameraMovement
  (params (Direction :type FP_CameraMovementDirection%20Enum :default "NewEnumerator0") (InputValue :type Float%20%28single-precision%29))
  (Default|OnCameraMovement (Variables|Default|GetPossessedPawn) Direction InputValue)
  (return))

(fn CheckInteractablesNearbyVisibility
  (bind _returnvalue (Viewport|GetViewportSize))
  (for _array_element (Variables|Default|GetInteractablesNearBy)
    (if (Math|Boolean|ANDBoolean (> (.x (.ScreenLocation (Class|PlayerController|ProjectWorldLocationtoScreen self (Transformation|GetActorLocation _array_element) false))) 0.0) (> (.y (.ScreenLocation (Class|PlayerController|ProjectWorldLocationtoScreen self (Transformation|GetActorLocation _array_element) false))) 0.0) (< (.x (.ScreenLocation (Class|PlayerController|ProjectWorldLocationtoScreen self (Transformation|GetActorLocation _array_element) false))) (.x _returnvalue)) (< (.y (.ScreenLocation (Class|PlayerController|ProjectWorldLocationtoScreen self (Transformation|GetActorLocation _array_element) false))) (.y _returnvalue)))
      (Development|PrintString (Utilities|GetDisplayName _array_element))
      (else
        (Development|PrintString "NOT VISIBLE")))))