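; Scene component that controls a child widget's visibility and hides it when the owning actor leaves the allowed screen area.
; BeginPlay caches the first child as a WidgetComponent and starts it hidden, printing the child's name if the cast fails.
; While activated, Tick projects the owner's location to screen and compares it to the available screen-space bounds.
; The bounds check only hides; showing goes through the toggle function.
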(event EventBeginPlay
  (bind _returnvalue (Components|GetChildComponent 0))
  (bind _aswidget_component (Utilities|Casting|CastToWidgetComponent _returnvalue)
    (:then
      (bind _output_get (Variables|Default|SetFP_WidgetComponent _aswidget_component))
      (Rendering|SetVisibility _output_get false true))
    (:CastFailed
      (Development|PrintString (Utilities|GetDisplayName _returnvalue)))))

(event EventTick
  (params (DeltaSeconds :type Float%20%28single-precision%29))
  (if (Variables|Default|GetFP_IsActivated)
    (CallFunction|FPScreenBoundsCheck)))

(fn FPToggleWidgetVisibility
  (params (NewParam :type Boolean))
  (bind _output_get (Variables|Default|SetFP_IsWidgetVisible NewParam))
  (Rendering|SetVisibility (Variables|Default|GetFP_WidgetComponent) _output_get true))

(fn FPScreenBoundsCheck
  (bind _returnvalue (Game|GetPlayerController 0))
  (bind _returnvalue_2 (Components|GetOwner))
  (bind _returnvalue_3 (Transformation|GetActorLocation _returnvalue_2))
  (bind _screenlocation (Class|PlayerController|ProjectWorldLocationtoScreen _returnvalue _returnvalue_3 false))
  (bind (_minx _maxx _miny _maxy) (CallFunction|FPGetAvailableScreenSpace))
  (bind _output_get (Variables|Default|SetFP_IsInScreenBounds (Math|Boolean|ANDBoolean (> (.x _screenlocation) _minx) (< (.x _screenlocation) _maxx) (> (.y _screenlocation) _miny) (< (.y _screenlocation) _maxy))))
  (if _output_get
    _
    (else
      (CallFunction|FPToggleWidgetVisibility false)))
  (return))